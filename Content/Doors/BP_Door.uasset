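; BP_Door is a hinged door that swings inward or outward by rotating its Hinge whenever the door alpha changes.
; CalculateAlpha uses a symmetrical ease if the door can be interacted with while moving, since asymmetrical curves would snap.
; Otherwise it samples one of four curve assets, chosen by GetCurve from open/close state and direction.
; GetDoorLocation reports the GraspableSphere's world position as the door's location.
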(event EventOnDoorAlphaChanged
  (params (OldDoorAlpha :type Float%20%28single-precision%29) (NewDoorAlpha :type Float%20%28single-precision%29) (State :type EDoorState%20Enum :default "Closed") (Direction :type EDoorDirection%20Enum :default "Outward") (DoorTime :type Float%20%28single-precision%29) (DoorTransitionTime :type Float%20%28single-precision%29))
  (bind _returnvalue (CallFunction|CalculateAlpha NewDoorAlpha State Direction DoorTime DoorTransitionTime))
  (Transformation|SetRelativeRotation (Variables|Default|GetHinge) (Utilities|Select :Index Direction :Outward (Math|Rotator|Lerp(Rotator) "0, 0, 0" "0.000000,90.000000,0.000000" _returnvalue true) :Inward (Math|Rotator|Lerp(Rotator) "0, 0, 0" "0.000000,-90.000000,0.000000" _returnvalue true)) false false))

(fn ConstructionScript)

(fn GetDoorLocation
  (return (Transformation|GetWorldLocation (Variables|Default|GetGraspableSphere))))

(fn GetCurve
  (params (State :type EDoorState%20Enum :default "Closed") (Direction :type EDoorDirection%20Enum :default "Outward"))
  (bind _returnvalue (Class|Door|IsDoorStateOpenorOpening State))
  (return (Utilities|Select :Index Direction :Outward (select _returnvalue (Variables|Default|GetDoorCurveOpenOutward) (Variables|Default|GetDoorCurveCloseOutward)) :Inward (select _returnvalue (Variables|Default|GetDoorCurveOpenInward) (Variables|Default|GetDoorCurveCloseInward)))))

(fn CalculateAlpha
  (params (NewAlpha :type Float%20%28double-precision%29) (State :type EDoorState%20Enum :default "Closed") (Direction :type EDoorDirection%20Enum :default "Outward") (Time :type Float%20%28double-precision%29) (TransitionTime :type Float%20%28single-precision%29))
  (return (Math|Float|SelectFloat (Math|Interpolation|Ease "EaseInOut" (Math|Float|Absolute(Float) NewAlpha) 1.0 0.0 6.0) (Math|Curves|GetFloatValue (CallFunction|GetCurve State Direction) (Math|Float|Absolute(Float) NewAlpha)) (Class|Door|CanInteractWhileinMotion))))