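; Sliding double door Blueprint that moves its left and right hinge components in opposite directions along local Y as the door alpha changes.
; Each alpha update lerps both hinges between mirrored offsets and the center using an eased alpha.
; Doors interactable while in motion use a symmetrical ease-in-out.
; Otherwise, separate open and close curve assets shape the motion, allowing asymmetrical curves that would snap if interrupted.
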(event EventOnDoorAlphaChanged
  (params (OldDoorAlpha :type Float%20%28single-precision%29) (NewDoorAlpha :type Float%20%28single-precision%29) (State :type EDoorState%20Enum :default "Closed") (Direction :type EDoorDirection%20Enum :default "Outward") (DoorTime :type Float%20%28single-precision%29) (DoorTransitionTime :type Float%20%28single-precision%29))
  (bind _returnvalue (CallFunction|CalculateAlpha NewDoorAlpha State Direction DoorTime DoorTransitionTime))
  (bind _returnvalue_2 (Math|Float|Absolute(Float) _returnvalue))
  (Transformation|SetRelativeLocation (Variables|Default|GetHingeL) (Math|Vector|Lerp(Vector) "0.000000,88.000000,10.000000" "0.000000,0.000000,10.000000" _returnvalue_2) false false)
  (Transformation|SetRelativeLocation (Variables|Default|GetHingeR) (Math|Vector|Lerp(Vector) "0.000000,-88.000000,10.000000" "0.000000,0.000000,10.000000" _returnvalue_2) false false))

(fn ConstructionScript)

(fn GetCurve
  (params (State :type EDoorState%20Enum :default "Closed") (Direction :type EDoorDirection%20Enum :default "Outward"))
  (return (select (Class|Door|IsDoorStateOpenorOpening State) (Variables|DoorVisuals|GetDoorCurveOpen) (Variables|DoorVisuals|GetDoorCurveClose))))

(fn CalculateAlpha
  (params (NewAlpha :type Float%20%28double-precision%29) (State :type EDoorState%20Enum :default "Closed") (Direction :type EDoorDirection%20Enum :default "Outward") (Time :type Float%20%28double-precision%29) (TransitionTime :type Float%20%28single-precision%29))
  (return (Math|Float|SelectFloat (Math|Interpolation|Ease "EaseInOut" (Math|Float|Absolute(Float) NewAlpha) 1.0 0.0 6.0) (Math|Curves|GetFloatValue (CallFunction|GetCurve State Direction) (Math|Float|Absolute(Float) NewAlpha)) (Class|Door|CanInteractWhileinMotion))))