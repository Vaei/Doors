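; Automatic door that opens when pawns overlap its OpenFront trigger and closes once the last one leaves.
; Overlaps maintain a HoldingDoor list and request state changes through a door ability check, retried when the cooldown finishes or the door state changes.
; Door alpha changes swing the hinge 90 degrees inward or outward, eased symmetrically if interruptible mid-motion, otherwise shaped by per-direction open/close curves, since asymmetrical curves would snap.
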(event OnComponentBeginOverlap(OpenFront)
  (params (OverlappedComponent :type Primitive%20Component%20Object%20Reference) (OtherActor :type Actor%20Object%20Reference) (OtherComp :type Primitive%20Component%20Object%20Reference) (OtherBodyIndex :type Integer) (bFromSweep :type Boolean) (SweepResult :type Hit%20Result%20Structure%20%28by%20ref%29))
  ;[1 1 1] Overlap events to open or close the door
  (bind _aspawn (Utilities|Casting|CastToPawn OtherActor))
  (Utilities|Array|AddUnique (Variables|Default|GetHoldingDoor) _aspawn)
  (CallFunction|OpenDoor _aspawn))

(event OnComponentEndOverlap(OpenFront)
  (params (OverlappedComponent :type Primitive%20Component%20Object%20Reference) (OtherActor :type Actor%20Object%20Reference) (OtherComp :type Primitive%20Component%20Object%20Reference) (OtherBodyIndex :type Integer))
  ;[1 1 1] Overlap events to open or close the door
  (bind _aspawn (Utilities|Casting|CastToPawn OtherActor))
  (Utilities|Array|RemoveItem (Variables|Default|GetHoldingDoor) _aspawn)
  (CallFunction|CloseDoor _aspawn))

(event Custom|CloseDoor
  (params (Avatar :type Object%20Object%20Reference))
  ;[1 1 1] Attempt to close the door
  (if (Class|Door|IsDoorOpenorOpening)
    (bind _aspawn (Utilities|Casting|CastToPawn Avatar))
    (Class|Door|SetLastAvatar _aspawn)
    (if (Utilities|Array|IsEmpty (Variables|Default|GetHoldingDoor))
      (bind _returnvalue (Class|Door|ShouldAbilityRespondtoDoorEvent _aspawn (Class|Door|GetDoorState) (Class|Door|GetDoorDirection) (Class|Door|GetDoorSide)))
      (if _returnvalue
        (Class|Door|SetDoorState "Closing" (Class|Door|GetDoorDirection) _aspawn)))))

(event Custom|OpenDoor
  (params (Avatar :type Object%20Object%20Reference))
  ;[1 1 1] Attempt to open the door
  (if (Class|Door|IsDoorClosedorClosing)
    (bind _aspawn (Utilities|Casting|CastToPawn Avatar))
    (Class|Door|SetLastAvatar _aspawn)
    (bind (_newdoorstate _newdoordirection _doormotion _failreason _returnvalue) (Class|Door|ShouldAbilityRespondtoDoorEvent _aspawn (Class|Door|GetDoorState) (Class|Door|GetDoorDirection) (Class|Door|GetDoorSide _aspawn)))
    (if _returnvalue
      (Class|Door|SetDoorState _newdoorstate _newdoordirection _aspawn))))

(event Custom|OnDoorCooldownFinished
  (params (Door :type Door%20Object%20Reference))
  ;[1 1 1] If we couldn't open or close the door because its on cooldown, we need to try again
  (CallFunction|TryCloseDoor)
  (CallFunction|TryOpenDoor))

(event Custom|TryCloseDoor
  ;[1 1 1] Try to close the door if we couldn't before
  (if (Class|Door|IsDoorStationary)
    (if (Utilities|Array|IsEmpty (Variables|Default|GetHoldingDoor))
      (CallFunction|CloseDoor (Class|Door|GetLastAvatar)))))

(event Custom|TryOpenDoor
  ;[1 1 1] Try to open the door if we couldn't before
  (if (Class|Door|IsDoorStationary)
    (if (Utilities|Array|IsNotEmpty (Variables|Default|GetHoldingDoor))
      (CallFunction|OpenDoor (Class|Door|GetLastAvatar)))))

(event EventOnDoorAlphaChanged
  (params (OldDoorAlpha :type Float%20%28single-precision%29) (NewDoorAlpha :type Float%20%28single-precision%29) (State :type EDoorState%20Enum :default "Closed") (Direction :type EDoorDirection%20Enum :default "Outward") (DoorTime :type Float%20%28single-precision%29) (DoorTransitionTime :type Float%20%28single-precision%29))
  (bind _returnvalue (CallFunction|CalculateAlpha NewDoorAlpha State Direction DoorTime DoorTransitionTime))
  ;[1 1 1] Perform the physical opening of the door mesh/collision
  (Transformation|SetRelativeRotation (Variables|Default|GetHinge) (Utilities|Select :Index Direction :Outward (Math|Rotator|Lerp(Rotator) "0, 0, 0" "0.000000,90.000000,0.000000" _returnvalue true) :Inward (Math|Rotator|Lerp(Rotator) "0, 0, 0" "0.000000,-90.000000,0.000000" _returnvalue true)) false false))

(event EventOnDoorStateChanged
  (params (OldDoorState :type EDoorState%20Enum :default "Closed") (NewDoorState :type EDoorState%20Enum :default "Closed") (OldDoorDirection :type EDoorDirection%20Enum :default "Outward") (NewDoorDirection :type EDoorDirection%20Enum :default "Outward") (Avatar :type Actor%20Object%20Reference) (bClientSimulation :type Boolean))
  ;[1 1 1] If the door was in motion and we can't change while in motion, try to change if it became stationary
  (CallFunction|TryCloseDoor)
  (CallFunction|TryOpenDoor))

(event EventBeginPlay
  ;[1 1 1] If we couldn't open or close the door because its on cooldown, we need to try again
  (EventDispatchers|AssignOnDoorCooldownFinishedDelegate (delegate Custom|OnDoorCooldownFinished)))

(fn ConstructionScript)

(fn GetCurve
  (params (State :type EDoorState%20Enum :default "Closed") (Direction :type EDoorDirection%20Enum :default "Outward"))
  (bind _returnvalue (Class|Door|IsDoorStateOpenorOpening State))
  (return (Utilities|Select :Index Direction :Outward (select _returnvalue (Variables|Default|GetDoorCurveOpenOutward) (Variables|Default|GetDoorCurveCloseOutward)) :Inward (select _returnvalue (Variables|Default|GetDoorCurveOpenInward) (Variables|Default|GetDoorCurveCloseInward)))))

(fn CalculateAlpha
  (params (NewAlpha :type Float%20%28double-precision%29) (State :type EDoorState%20Enum :default "Closed") (Direction :type EDoorDirection%20Enum :default "Outward") (Time :type Float%20%28double-precision%29) (TransitionTime :type Float%20%28single-precision%29))
  (return (Math|Float|SelectFloat (Math|Interpolation|Ease "EaseInOut" (Math|Float|Absolute(Float) NewAlpha) 1.0 0.0 6.0) (Math|Curves|GetFloatValue (CallFunction|GetCurve State Direction) (Math|Float|Absolute(Float) NewAlpha)) (Class|Door|CanInteractWhileinMotion))))